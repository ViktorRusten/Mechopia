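; Mr Mushy Bolt enemy that chases the player and damages them on contact.
; Tick sends it toward the player through its instigator controller with SimpleMoveToActor.
; On overlap, if it touches the player it calls DealDamage and prints the result.
; Hit or death sounds play, chosen by Dead, only when the overlapping actor is a PlayerBullet3_BP and the player is also overlapping.
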(event Collision|EventActorBeginOverlap
  (params (OtherActor :type Actor%20Object%20Reference))
  (bind _returnvalue (Game|GetPlayerCharacter 0))
  (bind _self self)
  (bind _returnvalue_2 (Transformation|GetActorLocation _self))
  ;[1 1 1] Dealing damage
  (if (Collision|IsOverlappingActor _returnvalue :!class /Script/Engine.Actor)
    (if true
      (Utilities|Casting|CastToMechopiaCharacter _returnvalue
        (:then
          (bind _output_get (Variables|Default|SetNewVar_0 (Class|MrMushy|DealDamage self)))
          (Development|PrintText (Utilities|Text|ToText(Integer) _output_get) false))
        (:CastFailed
          _))
      ;[1 1 1] Playing sound from getting hit
      (Utilities|Casting|CastToPlayerBullet3_BP OtherActor)
      (if (Variables|Default|GetDead)
        (Audio|PlaySoundatLocation "/Game/Audio/DeathEnemies.DeathEnemies" _returnvalue_2)
        (else
          (Audio|PlaySoundatLocation "/Game/Audio/EnemyHit.EnemyHit" _returnvalue_2))))))

(event EventTick
  (params (DeltaSeconds :type Float%20%28single-precision%29))
  (bind _returnvalue (Game|GetPlayerCharacter 0))
  ;[1 1 1] Movement
  (Utilities|IsValid _returnvalue
    (:Is%20Valid
      (AI|Navigation|SimpleMovetoActor (Game|GetInstigatorController) _returnvalue))))

(event EventBeginPlay
  ;[1 1 1] Setting a reference to the player
  (Variables|Default|SetThePlayerActor (Game|GetPlayerCharacter 0)))

(fn ConstructionScript)