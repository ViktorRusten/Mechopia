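; Big switch Blueprint that ends the current level and loads StartLevel once activated.
; Tick polls the Active flag, which is not set in this file, and uses a DoOnce to fire the sequence a single time.
; The sequence plays a power-up sound at the world origin, starts a held camera fade-out, then opens the level after a short delay.
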(event EventBeginPlay
  (|CallParentFunction))

(event Collision|EventActorBeginOverlap
  (params (OtherActor :type Actor%20Object%20Reference)))

(event EventTick
  (params (DeltaSeconds :type Float%20%28single-precision%29))
  (|CallParentFunction 0.0)
  (if (Variables|Default|GetActive)
    (Utilities|FlowControl|DoOnce false
      (:Completed
        (Audio|PlaySoundatLocation "/Game/Audio/Power_Up_02.Power_Up_02" "0, 0, 0")
        (CameraFades|StartCameraFade :self (Game|GetPlayerCameraManager 0) :ToAlpha 1.0 :Duration 2.5 :bHoldWhenFinished true)
        (Utilities|FlowControl|Delay 4.0)
        (Game|OpenLevel(byName) "StartLevel")))))

(fn ConstructionScript
  (|CallParentFunction))